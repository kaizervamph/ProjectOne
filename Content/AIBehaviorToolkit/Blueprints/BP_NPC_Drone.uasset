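; BP_NPC_Drone is an NPC drone whose spotlight blinks and changes color to show its AI behavior state.
; A looping timer set at BeginPlay toggles the spotlight's visibility at the BlinkTime interval.
; BehaviorComponent events tint the light red for follow, near-white for patrol and red-orange for investigate.
; Investigate also shortens BlinkTime, but the running timer is not restarted, so its rate is unchanged.
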(event `self.ReceiveBeginPlay`
  (`parent.ReceiveBeginPlay`)
  (`self.Blink`))

(event `self.ReceiveTick`
  (params (DeltaSeconds :type "Float (single-precision)")))

(event `Blink`
  (`KismetSystemLibrary.K2_SetTimerDelegate` (delegate `SetLightVisibility`) (`self.BlinkTime`) true))

(event `SetLightVisibility`
  (bind _spotlight (`self.SpotLight`))
  (`SceneComponent.SetVisibility` _spotlight (not (`SceneComponent.bVisible` _spotlight)) false))

(event `self.BehaviorComponent.OnBeginFollow`
  (`LightComponent.SetLightColor` (`self.SpotLight`) (struct :`R` 0.895833 :`A` 1.0) true))

(event `self.BehaviorComponent.OnBeginPatrol`
  (`LightComponent.SetLightColor` (`self.SpotLight`) (struct :`R` 1.0 :`G` 0.98702 :`B` 0.976708 :`A` 1.0) true))

(event `self.BehaviorComponent.OnBeginAttackMelee`)

(event `self.BehaviorComponent.OnBeginInvestigate`
  (set `self.BlinkTime` 0.2)
  (`LightComponent.SetLightColor` (`self.SpotLight`) (struct :`R` 0.895833 :`G` 0.122621 :`A` 1.0) true))

(fn `UserConstructionScript`
  (`parent.UserConstructionScript`))